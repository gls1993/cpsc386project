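; BP_Road is a road lane actor that builds a strip of road meshes along its Y axis in the construction script and populates it with traffic and coins.
; On BeginPlay it scatters random coins between the Start and End points, picks one travel direction and starts a looping timer with a randomized interval.
; Each tick of that timer may spawn a car at the chosen end, and overlap volumes at both ends destroy cars.
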(event `SpawnCars`
  (if (`KismetMathLibrary.RandomBool`)
    (if (`self.startingcarlocation`)
      (`|SpawnActorFromClass` "/Game/Blueprints/BP_Cars.BP_Cars_C" (`KismetMathLibrary.MakeTransform` (`self.StartLocation`) (struct :`Yaw` 90.0)) "Undefined" "OverrideRootScale" null null)
      (else
        (`|SpawnActorFromClass` "/Game/Blueprints/BP_Cars.BP_Cars_C" (`KismetMathLibrary.MakeTransform` (`self.EndLocation`) (struct :`Yaw` -90.0)) "Undefined" "OverrideRootScale" null null)))))

(event `self.ReceiveBeginPlay`
  (bind (_startlocation_x _startlocation_y _startlocation_z) (`KismetMathLibrary.BreakVector` (`self.StartLocation`)))
  (`|ExecutionSequence`
    (:`then_0`
      (set `self.StartLocation` (`SceneComponent.K2_GetComponentLocation` (`self.start`)))
      (set `self.EndLocation` (`SceneComponent.K2_GetComponentLocation` (`self.end`)))
      (for _index (range (+ (`KismetMathLibrary.FTrunc` (/ (`KismetMathLibrary.Vector_Distance` (`self.StartLocation`) (`self.EndLocation`)) 250.0)) 1))
        (if (> (`KismetMathLibrary.RandomFloat`) 0.8)
          (`|SpawnActorFromClass` "/Game/Blueprints/BP_Coins.BP_Coins_C" (`KismetMathLibrary.MakeTransform` (`KismetMathLibrary.MakeVector` _startlocation_x (+ (`KismetMathLibrary.Conv_IntToDouble` (* _index 250)) (`KismetMathLibrary.Conv_IntToDouble` (`KismetMathLibrary.FTrunc` (.y (`self.StartLocation`))))) _startlocation_z)) "Undefined" "OverrideRootScale" null null))))
    (:`then_1`
      (set `self.StartLocation` (`SceneComponent.K2_GetComponentLocation` (`self.start`)))
      (set `self.EndLocation` (`SceneComponent.K2_GetComponentLocation` (`self.end`)))
      (set `self.startingcarlocation` (`KismetMathLibrary.RandomBool`))
      (`KismetSystemLibrary.K2_SetTimerDelegate` (delegate `SpawnCars`) (`KismetMathLibrary.RandomFloatInRange` 2.0 10.0) true))))

(event `self.Hitstart.OnComponentBeginOverlap`
  (params (OverlappedComponent :type "PrimitiveComponent Object Reference") (OtherActor :type "Actor Object Reference") (OtherComp :type "PrimitiveComponent Object Reference") (OtherBodyIndex :type Integer) (bFromSweep :type Boolean) (SweepResult :type "HitResult Structure (by ref)"))
  (bind _asbp_cars (cast `/Game/Blueprints/BP_Cars` OtherActor))
  (`self.K2_DestroyActor` _asbp_cars))

(event `self.Hitend.OnComponentBeginOverlap`
  (params (OverlappedComponent :type "PrimitiveComponent Object Reference") (OtherActor :type "Actor Object Reference") (OtherComp :type "PrimitiveComponent Object Reference") (OtherBodyIndex :type Integer) (bFromSweep :type Boolean) (SweepResult :type "HitResult Structure (by ref)"))
  (bind _asbp_cars (cast `/Game/Blueprints/BP_Cars` OtherActor))
  (`self.K2_DestroyActor` _asbp_cars))

(fn `UserConstructionScript`
  (for _index (range 101)
    (bind _returnvalue (`AddComponent|NODE_AddStaticMeshComponent-0`))
    (`StaticMeshComponent.SetStaticMesh` _returnvalue "/Game/Roads/unmarkedRoad.unmarkedRoad")
    (`SceneComponent.K2_SetRelativeLocationAndRotation` :`self` _returnvalue :`NewLocation` (`KismetMathLibrary.MakeVector` 0.0 (* (`KismetMathLibrary.Conv_IntToDouble` _index) 80.0) 80.0))))