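; BP_Water is a river lane for a chicken crossing game that spawns floating logs and makes the chicken fall in on overlap.
; Its construction script builds the lane from a row of water meshes.
; At BeginPlay it picks one travel direction and starts a looping timer with a randomized period, each tick having a coin-flip chance to spawn a Log_Spawner1.
; Trigger volumes destroy arriving logs, while the water box calls Fallinwater once.
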(event `SpawnCars`
  (if (`KismetMathLibrary.RandomBool`)
    (if (`self.startingcarlocation`)
      (`|SpawnActorFromClass` "/Game/Blueprints/Log_Spawner1.Log_Spawner1_C" (`KismetMathLibrary.MakeTransform` (`self.StartLocation`) (struct :`Yaw` 90.0)) "Undefined" "OverrideRootScale" null null)
      (else
        (`|SpawnActorFromClass` "/Game/Blueprints/Log_Spawner1.Log_Spawner1_C" (`KismetMathLibrary.MakeTransform` (`self.EndLocation`) (struct :`Yaw` -90.0)) "Undefined" "OverrideRootScale" null null)))))

(event `self.ReceiveBeginPlay`
  (set `self.StartLocation` (`SceneComponent.K2_GetComponentLocation` (`self.start`)))
  (set `self.EndLocation` (`SceneComponent.K2_GetComponentLocation` (`self.end`)))
  (set `self.startingcarlocation` (`KismetMathLibrary.RandomBool`))
  (`KismetSystemLibrary.K2_SetTimerDelegate` (delegate `SpawnCars`) (`KismetMathLibrary.RandomFloatInRange` 2.0 3.0) true))

(event `self.Box.OnComponentBeginOverlap`
  (params (OverlappedComponent :type "PrimitiveComponent Object Reference") (OtherActor :type "Actor Object Reference") (OtherComp :type "PrimitiveComponent Object Reference") (OtherBodyIndex :type Integer) (bFromSweep :type Boolean) (SweepResult :type "HitResult Structure (by ref)"))
  (bind _aschicken_character (cast `/Game/Blueprints/ChickenCharacter` OtherActor))
  (`/Engine/EditorBlueprintResources/StandardMacros.DoOnce` false
    (:`Completed`
      (`/Game/Blueprints/ChickenCharacter.Fallinwater` _aschicken_character))))

(event `self.Hitstart.OnComponentBeginOverlap`
  (params (OverlappedComponent :type "PrimitiveComponent Object Reference") (OtherActor :type "Actor Object Reference") (OtherComp :type "PrimitiveComponent Object Reference") (OtherBodyIndex :type Integer) (bFromSweep :type Boolean) (SweepResult :type "HitResult Structure (by ref)"))
  (bind _aslog_spawner_1 (cast `/Game/Blueprints/Log_Spawner1` OtherActor))
  (`self.K2_DestroyActor` _aslog_spawner_1))

(event `self.Hitend.OnComponentBeginOverlap`
  (params (OverlappedComponent :type "PrimitiveComponent Object Reference") (OtherActor :type "Actor Object Reference") (OtherComp :type "PrimitiveComponent Object Reference") (OtherBodyIndex :type Integer) (bFromSweep :type Boolean) (SweepResult :type "HitResult Structure (by ref)"))
  (bind _aslog_spawner_1 (cast `/Game/Blueprints/Log_Spawner1` OtherActor))
  (`self.K2_DestroyActor` _aslog_spawner_1))

(fn `UserConstructionScript`
  (for _index (range 101)
    (bind _returnvalue (`AddComponent|NODE_AddStaticMeshComponent-0`))
    (`StaticMeshComponent.SetStaticMesh` _returnvalue "/Game/Waterfall/waterbrightBase.waterbrightBase")
    (`SceneComponent.K2_SetRelativeLocationAndRotation` :`self` _returnvalue :`NewLocation` (`KismetMathLibrary.MakeVector` 0.0 (* (`KismetMathLibrary.Conv_IntToDouble` _index) 80.0) 80.0))))