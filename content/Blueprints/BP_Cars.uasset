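; BP_Cars is a car obstacle that hits the player's chicken character.
; On BeginPlay it randomly swaps the Car mesh to one of four vehicle models, or keeps the default mesh on a roll of zero.
; An overlap on its Box casts to ChickenCharacter and calls HitbyCar, gated by a DoOnce that is never reset, so each car hits only once.
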(event `self.ReceiveBeginPlay`
  (switch `int` (`KismetMathLibrary.RandomIntegerInRange` 0 4)
    (:`1`
      (`StaticMeshComponent.SetStaticMesh` (`self.car`) "/Game/Vehicles/FedExTruck.FedExTruck"))
    (:`2`
      (`StaticMeshComponent.SetStaticMesh` (`self.car`) "/Game/Vehicles/long_car_Rolls_Royce.long_car_Rolls_Royce"))
    (:`3`
      (`StaticMeshComponent.SetStaticMesh` (`self.car`) "/Game/Vehicles/pizza_car_Untitled.pizza_car_Untitled"))
    (:`4`
      (`StaticMeshComponent.SetStaticMesh` (`self.car`) "/Game/Vehicles/policeCar.policeCar"))))

(event `self.Box.OnComponentBeginOverlap`
  (params (OverlappedComponent :type "PrimitiveComponent Object Reference") (OtherActor :type "Actor Object Reference") (OtherComp :type "PrimitiveComponent Object Reference") (OtherBodyIndex :type Integer) (bFromSweep :type Boolean) (SweepResult :type "HitResult Structure (by ref)"))
  (bind _aschicken_character (cast `/Game/Blueprints/ChickenCharacter` OtherActor))
  (`/Engine/EditorBlueprintResources/StandardMacros.DoOnce` false
    (:`Completed`
      (`/Game/Blueprints/ChickenCharacter.HitbyCar` _aschicken_character))))

(fn `UserConstructionScript`)