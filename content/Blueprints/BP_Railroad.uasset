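; Railroad track actor that periodically sends trains along its length in a direction chosen randomly at BeginPlay.
; The construction script lays repeated rail meshes along local Y.
; A looping timer, its interval randomized once, gives a coin-flip chance to spawn a front piece, four cars and a rear piece, staggered by delays, from the Start or End marker.
; Hitstart and Hitend overlaps destroy any train pieces that enter them.
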(event `self.ReceiveBeginPlay`
  (set `self.StartLocation` (`SceneComponent.K2_GetComponentLocation` (`self.start`)))
  (set `self.EndLocation` (`SceneComponent.K2_GetComponentLocation` (`self.end`)))
  (set `self.startingtrainlocation` (`KismetMathLibrary.RandomBool`))
  (`KismetSystemLibrary.K2_SetTimerDelegate` (delegate `Spawn Train`) (`KismetMathLibrary.RandomFloatInRange` 8.0 10.0) true))

(event `Spawn Train`
  (bind _startlocation (`self.StartLocation`))
  (bind _endlocation (`self.EndLocation`))
  (if (`KismetMathLibrary.RandomBool`)
    (if (`self.startingtrainlocation`)
      (`|SpawnActorFromClass` "/Game/Blueprints/trainspawner.trainspawner_C" (`KismetMathLibrary.MakeTransform` _startlocation (struct :`Yaw` 90.0)) "Undefined" "OverrideRootScale" null null)
      (`KismetSystemLibrary.Delay` 1.25)
      (`|SpawnActorFromClass` "/Game/Blueprints/traincarspawner.traincarspawner_C" (`KismetMathLibrary.MakeTransform` _startlocation (struct :`Yaw` 90.0)) "Undefined" "OverrideRootScale" null null)
      (`KismetSystemLibrary.Delay` 1.25)
      (`|SpawnActorFromClass` "/Game/Blueprints/traincarspawner.traincarspawner_C" (`KismetMathLibrary.MakeTransform` _startlocation (struct :`Yaw` 90.0)) "Undefined" "OverrideRootScale" null null)
      (`KismetSystemLibrary.Delay` 1.25)
      (`|SpawnActorFromClass` "/Game/Blueprints/traincarspawner.traincarspawner_C" (`KismetMathLibrary.MakeTransform` _startlocation (struct :`Yaw` 90.0)) "Undefined" "OverrideRootScale" null null)
      (`KismetSystemLibrary.Delay` 1.25)
      (`|SpawnActorFromClass` "/Game/Blueprints/traincarspawner.traincarspawner_C" (`KismetMathLibrary.MakeTransform` _startlocation (struct :`Yaw` 90.0)) "Undefined" "OverrideRootScale" null null)
      (`KismetSystemLibrary.Delay` 1.25)
      (`|SpawnActorFromClass` "/Game/Blueprints/trainspawnerR.trainspawnerR_C" (`KismetMathLibrary.MakeTransform` _startlocation (struct :`Yaw` 90.0)) "Undefined" "OverrideRootScale" null null)
      (else
        (`|SpawnActorFromClass` "/Game/Blueprints/trainspawner.trainspawner_C" (`KismetMathLibrary.MakeTransform` _endlocation (struct :`Yaw` -90.0)) "Undefined" "OverrideRootScale" null null)
        (`KismetSystemLibrary.Delay` 1.25)
        (`|SpawnActorFromClass` "/Game/Blueprints/traincarspawner.traincarspawner_C" (`KismetMathLibrary.MakeTransform` _endlocation (struct :`Yaw` -90.0)) "Undefined" "OverrideRootScale" null null)
        (`KismetSystemLibrary.Delay` 1.25)
        (`|SpawnActorFromClass` "/Game/Blueprints/traincarspawner.traincarspawner_C" (`KismetMathLibrary.MakeTransform` _endlocation (struct :`Yaw` -90.0)) "Undefined" "OverrideRootScale" null null)
        (`KismetSystemLibrary.Delay` 1.25)
        (`|SpawnActorFromClass` "/Game/Blueprints/traincarspawner.traincarspawner_C" (`KismetMathLibrary.MakeTransform` _endlocation (struct :`Yaw` -90.0)) "Undefined" "OverrideRootScale" null null)
        (`KismetSystemLibrary.Delay` 1.25)
        (`|SpawnActorFromClass` "/Game/Blueprints/traincarspawner.traincarspawner_C" (`KismetMathLibrary.MakeTransform` _endlocation (struct :`Yaw` -90.0)) "Undefined" "OverrideRootScale" null null)
        (`KismetSystemLibrary.Delay` 1.25)
        (`|SpawnActorFromClass` "/Game/Blueprints/trainspawnerR.trainspawnerR_C" (`KismetMathLibrary.MakeTransform` _endlocation (struct :`Yaw` -90.0)) "Undefined" "OverrideRootScale" null null)))))

(event `self.Hitstart.OnComponentBeginOverlap`
  (params (OverlappedComponent :type "PrimitiveComponent Object Reference") (OtherActor :type "Actor Object Reference") (OtherComp :type "PrimitiveComponent Object Reference") (OtherBodyIndex :type Integer) (bFromSweep :type Boolean) (SweepResult :type "HitResult Structure (by ref)"))
  (bind _astrainspawner (cast `/Game/Blueprints/trainspawner` OtherActor)
    (:`then`
      _)
    (:`CastFailed`
      (bind _astraincarspawner (cast `/Game/Blueprints/traincarspawner` OtherActor)
        (:`then`
          _)
        (:`CastFailed`
          (bind _astrainspawner_r (cast `/Game/Blueprints/trainspawnerR` OtherActor))))))
  (`self.K2_DestroyActor` _astrainspawner)
  (`self.K2_DestroyActor` _astraincarspawner)
  (`self.K2_DestroyActor` _astrainspawner_r))

(event `self.Hitend.OnComponentBeginOverlap`
  (params (OverlappedComponent :type "PrimitiveComponent Object Reference") (OtherActor :type "Actor Object Reference") (OtherComp :type "PrimitiveComponent Object Reference") (OtherBodyIndex :type Integer) (bFromSweep :type Boolean) (SweepResult :type "HitResult Structure (by ref)"))
  (bind _astrainspawner (cast `/Game/Blueprints/trainspawner` OtherActor)
    (:`then`
      _)
    (:`CastFailed`
      (bind _astraincarspawner (cast `/Game/Blueprints/traincarspawner` OtherActor)
        (:`then`
          _)
        (:`CastFailed`
          (bind _astrainspawner_r (cast `/Game/Blueprints/trainspawnerR` OtherActor))))))
  (`self.K2_DestroyActor` _astrainspawner)
  (`self.K2_DestroyActor` _astraincarspawner)
  (`self.K2_DestroyActor` _astrainspawner_r))

(fn `UserConstructionScript`
  (for _index (range 101)
    (bind _returnvalue (`AddComponent|NODE_AddStaticMeshComponent-0`))
    (`StaticMeshComponent.SetStaticMesh` _returnvalue "/Game/Roads/newrailroad.newrailroad")
    (`SceneComponent.K2_SetRelativeLocationAndRotation` :`self` _returnvalue :`NewLocation` (`KismetMathLibrary.MakeVector` 0.0 (* (`KismetMathLibrary.Conv_IntToDouble` _index) 80.0) 80.0))))